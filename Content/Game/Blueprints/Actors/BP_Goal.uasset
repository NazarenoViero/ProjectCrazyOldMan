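; BP_Goal is the finish line actor that counts player laps and ends the game.
; When its checkpoint component allows interaction, an overlapping player not already in PlayersCrossed is added and gains a lap.
; Reaching that player's lap total shows a win widget on their screen, then loads the menu after a delay.
; Otherwise it clears registered players from every checkpoint; PlayersCrossed is never cleared here.
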(event EventBeginPlay
  (bind _returnvalue (UserInterface|CreateWidget "/Game/Game/Blueprints/Widget/WBP_WinGame.WBP_WinGame_C" (Game|GetPlayerController 0)))
  (Variables|Default|SetWBP_Win _returnvalue)
  (bind _asgi_cerebro_juego (Utilities|Casting|CastToGI_CerebroJuego (Game|GetGameInstance)))
  (Variables|Default|SetTotalLaps (Variables|/Game/Game/GameMode/GameInstance/GI_CerebroJuego.GI_CerebroJuego_C|GetVueltasTotalesElegidas _asgi_cerebro_juego)))

(event Collision|EventActorBeginOverlap
  (params (OtherActor :type Actor%20Object%20Reference))
  (bind _asbp_player_character (Utilities|Casting|CastToBP_PlayerCharacter OtherActor))
  (bind _output_get (Variables|Default|SetAs%20BP%20Player%20Character _asbp_player_character))
  (if (Variables|/Game/Game/Blueprints/Components/BPC_TakeCheckpoints.BPC_TakeCheckpoints_C|GetbCanInteract? (Variables|Default|GetBPC_TakeCheckpoints))
    (if (not (Utilities|Array|ContainsItem (Variables|Default|GetPlayersCrossed) (Variables|Default|GetAs%20BP%20Player%20Character)))
      (Utilities|Array|Add (Variables|Default|GetPlayersCrossed) (Variables|Default|GetAs%20BP%20Player%20Character))
      (bind _result (Math|Integer|IncrementInt (Variables|/Game/Game/Blueprints/Characters/BP_PlayerCharacter.BP_PlayerCharacter_C|GetVueltasActuales (Variables|Default|GetAs%20BP%20Player%20Character)))
        (:%20%20
          (if (== _result (Variables|/Game/Game/Blueprints/Characters/BP_PlayerCharacter.BP_PlayerCharacter_C|GetVueltasTotales (Variables|Default|GetAs%20BP%20Player%20Character)))
            (bind _returnvalue (UserInterface|CreateWidget "/Game/Game/Blueprints/Widget/WBP_WinGame.WBP_WinGame_C" (Variables|/Game/Game/Blueprints/Characters/BP_PlayerCharacter.BP_PlayerCharacter_C|GetRefPlayerController _output_get)))
            (UserInterface|Viewport|AddtoPlayerScreen _returnvalue)
            (Utilities|FlowControl|Delay 5.0)
            (Game|OpenLevel(byName) "LVL_Menu")
            (else
              (for _array_element (Variables|/Game/Game/Blueprints/Components/BPC_TakeCheckpoints.BPC_TakeCheckpoints_C|GetCheckpointsTotal (Variables|Default|GetBPC_TakeCheckpoints))
                (Utilities|Array|Clear (Variables|/Game/Game/Blueprints/Actors/BP_Checkpoint.BP_Checkpoint_C|GetPlayersRegistered _array_element))))))))))

(event EventTick
  (params (DeltaSeconds :type Float%20%28single-precision%29)))

(fn ConstructionScript)