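; BPC_TakeCheckpoints is a component that unlocks interaction once every checkpoint in its list has been taken.
; On BeginPlay it stores the size of CheckpointsTotal and binds its Taking event to each checkpoint's TakeCheckpoint event.
; Each Taking call increments CheckpointsTaken and sets CanInteract to true when the count reaches the total, so no Tick polling is used.
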(event Custom|Taking
  (bind _result (Math|Integer|IncrementInt (Variables|Default|GetCheckpointsTaken))
    (:%20%20
      (if (== _result (Variables|Default|GetCheckpointsToTake))
        (Variables|Default|SetbCanInteract? true)))))

(event EventBeginPlay
  (Variables|Default|SetCheckpointsToTake (Utilities|Array|Length (Variables|Default|GetCheckpointsTotal)))
  (for _array_element (Variables|Default|GetCheckpointsTotal)
    (EventDispatchers|BindEventtoTakeCheckpoint _array_element (delegate Custom|Taking))))

(event EventTick
  (params (DeltaSeconds :type Float%20%28single-precision%29)))