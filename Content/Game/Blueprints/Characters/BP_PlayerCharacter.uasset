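; Player car pawn for a sprite-based racing game with local two-player support, laps read from the game instance, a HUD and a coin component.
; Enhanced Input sets throttle and yaw, which Tick turns into swept movement with clamped speed and friction.
; P2 actions are forwarded to player pawn 1, so one local controller drives both cars.
; Car sprite follows the spawned-car count; hits reverse speed against cars and dampen it otherwise.
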(event Custom|Update_Custom_Acceleration
  (params (AxisValue :type Float%20%28double-precision%29))
  (if (Variables|Movement|GetbPuedeMoverse)
    (Variables|Movement|SetInputAceleration AxisValue)))

(event Custom|Update%20Custom%20Rotation
  (params (Axis%20Value :type Float%20%28double-precision%29))
  (if (Variables|Movement|GetbPuedeMoverse)
    (Transformation|AddActorLocalRotation (Math|Rotator|MakeRotator 0.0 0.0 (* (* Axis%20Value (Variables|Movement|GetTurnRate)) (Utilities|Time|GetWorldDeltaSeconds))) false false)))

(event Input|EnhancedActionEvents|EnhancedInputActionIA_Acceleration_P1
  (params (ActionValue :type Float%20%28double-precision%29) (ElapsedSeconds :type Float%20%28double-precision%29) (TriggeredSeconds :type Float%20%28double-precision%29) (InputAction :type Input%20Action%20Object%20Reference :default "/Game/Game/Blueprints/Characters/MappingContext/Inputs/IA_Acceleration_P1.IA_Acceleration_P1"))
  (:Triggered
    (CallFunction|UpdateCustomAcceleration ActionValue))
  (:Completed
    (CallFunction|UpdateCustomAcceleration 0.0)))

(event Input|EnhancedActionEvents|EnhancedInputActionIA_Rotation_P1
  (params (ActionValue :type Float%20%28double-precision%29) (ElapsedSeconds :type Float%20%28double-precision%29) (TriggeredSeconds :type Float%20%28double-precision%29) (InputAction :type Input%20Action%20Object%20Reference :default "/Game/Game/Blueprints/Characters/MappingContext/Inputs/IA_Rotation_P1.IA_Rotation_P1"))
  (CallFunction|UpdateCustomRotation ActionValue))

(event Input|EnhancedActionEvents|EnhancedInputActionIA_Acceleration_P2
  (params (ActionValue :type Float%20%28double-precision%29) (ElapsedSeconds :type Float%20%28double-precision%29) (TriggeredSeconds :type Float%20%28double-precision%29) (InputAction :type Input%20Action%20Object%20Reference :default "/Game/Game/Blueprints/Characters/MappingContext/Inputs/IA_Acceleration_P2.IA_Acceleration_P2"))
  (bind _returnvalue (Pawn|IsLocallyControlled))
  (bind _returnvalue_2 (Game|Player|GetPlayerPawn 1))
  (:Triggered
    (if _returnvalue
      (bind _asbp_player_character (Utilities|Casting|CastToBP_PlayerCharacter _returnvalue_2))
      (CallFunction|UpdateCustomAcceleration _asbp_player_character ActionValue)))
  (:Completed
    (if _returnvalue
      (bind _asbp_player_character_2 (Utilities|Casting|CastToBP_PlayerCharacter _returnvalue_2))
      (CallFunction|UpdateCustomAcceleration _asbp_player_character_2 0.0))))

(event Input|EnhancedActionEvents|EnhancedInputActionIA_Rotation_P2
  (params (ActionValue :type Float%20%28double-precision%29) (ElapsedSeconds :type Float%20%28double-precision%29) (TriggeredSeconds :type Float%20%28double-precision%29) (InputAction :type Input%20Action%20Object%20Reference :default "/Game/Game/Blueprints/Characters/MappingContext/Inputs/IA_Rotation_P2.IA_Rotation_P2"))
  (if (Pawn|IsLocallyControlled)
    (bind _asbp_player_character (Utilities|Casting|CastToBP_PlayerCharacter (Game|Player|GetPlayerPawn 1)))
    (CallFunction|UpdateCustomRotation _asbp_player_character ActionValue)))

(event EventBeginPlay
  (bind _asplayer_controller (Utilities|Casting|CastToPlayerController (Pawn|GetController)))
  (Variables|Default|SetRefPlayerController _asplayer_controller)
  (Input|AddMappingContext (PlayerController|LocalPlayerSubsystems|GetEnhancedInputLocalPlayerSubsystem _asplayer_controller) "/Game/Game/Blueprints/Characters/MappingContext/IMC_Inputs.IMC_Inputs" 0 "(bIgnoreAllPressedKeysUntilRelease=True,bForceImmediately=False,bNotifyUserSettings=False)")
  (bind _outactors (Actor|GetAllActorsOfClass "BP_PlayerCharacter_C"))
  (bind _output_get (Variables|Default|SetPlayerID (Utilities|Array|Length _outactors)))
  (switch int _output_get
    (:0
      (Rendering|Components|Sprite|SetSprite (Variables|Default|GetPaperSprite) "/Game/Game/Assets/Cars/Auto1_con_la_ranita_mejorada_Sprite_0.Auto1_con_la_ranita_mejorada_Sprite_0" :!label _label))
    (:1
      (goto _label))
    (:2
      (Rendering|Components|Sprite|SetSprite (Variables|Default|GetPaperSprite) "/Game/Game/Assets/Cars/Auto_2_Sprite.Auto_2_Sprite"))))

(event Collision|EventHit
  (params (MyComp :type Primitive%20Component%20Object%20Reference) (Other :type Actor%20Object%20Reference) (OtherComp :type Primitive%20Component%20Object%20Reference) (bSelfMoved :type Boolean) (HitLocation :type Vector :default "0, 0, 0") (HitNormal :type Vector :default "0, 0, 0") (NormalImpulse :type Vector :default "0, 0, 0") (Hit :type Hit%20Result%20Structure%20%28by%20ref%29))
  (Utilities|Casting|CastToBP_PlayerCharacter Other
    (:then
      (Variables|Movement|SetCurrentSpeed (* (Variables|Movement|GetCurrentSpeed) -1.0)))
    (:CastFailed
      (Variables|Movement|SetCurrentSpeed (* (Variables|Movement|GetCurrentSpeed) 0.8)))))

(event EventTick
  (params (DeltaSeconds :type Float%20%28single-precision%29))
  (bind _inputaceleration (Variables|Movement|GetInputAceleration))
  (if (!= 0.0 _inputaceleration)
    (Variables|Movement|SetCurrentSpeed (Math|Float|Clamp(Float) (+ (Variables|Movement|GetCurrentSpeed) (* (* _inputaceleration (Utilities|Time|GetWorldDeltaSeconds)) (Variables|Movement|GetAcceleration))) (Variables|Movement|GetMaxReverseSpeed) (Variables|Movement|GetMaxSpeed)))
    (else
      (Variables|Movement|SetCurrentSpeed (Math|Interpolation|FInterpTo (Variables|Movement|GetCurrentSpeed) 0.0 (Utilities|Time|GetWorldDeltaSeconds) (Variables|Movement|GetFriction)))))
  (Transformation|AddActorWorldOffset (* (* (Transformation|GetActorForwardVector) (Variables|Movement|GetCurrentSpeed)) (Utilities|Time|GetWorldDeltaSeconds)) true))

(event EventPossessed
  (params (NewController :type Controller%20Object%20Reference))
  (bind _asgi_cerebro_juego (Utilities|Casting|CastToGI_CerebroJuego (Game|GetGameInstance)))
  (Variables|Default|SetVueltasTotales (Variables|/Game/Game/GameMode/GameInstance/GI_CerebroJuego.GI_CerebroJuego_C|GetVueltasTotalesElegidas _asgi_cerebro_juego))
  (bind _asplayer_controller (Utilities|Casting|CastToPlayerController NewController))
  (Variables|Default|SetRefPlayerController _asplayer_controller)
  (if (Pawn|IsLocallyControlled)
    (bind _returnvalue (UserInterface|CreateWidget "/Game/Game/Blueprints/Widget/WBP_HUD.WBP_HUD_C" (Variables|Default|GetRefPlayerController)))
    (UserInterface|Viewport|AddtoPlayerScreen _returnvalue)))

(event EventAddCoins
  (params (CoinsToAdd :type Integer))
  (Default|AddCoins (Variables|Default|GetBPC_Coins) CoinsToAdd))

(fn ConstructionScript)